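; BP_Zombie is a damageable zombie with a health widget held in a 3D widget component.
; On BeginPlay it passes itself to that ZombieHP widget as its Zombie reference.
; Each AnyDamage event shrinks the actor's scale by a tenth and subtracts the damage from HP, destroying the actor once HP is nearly zero or below.
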(event `self.ReceiveBeginPlay`
  (bind _aszombie_hp (cast `/Game/LEC091011/ZombieHP` (`WidgetComponent.GetWidget` (`self.3D Widget Holding Component`))))
  (set `/Game/LEC091011/ZombieHP.Zombie` self _aszombie_hp))

(event `self.ReceiveAnyDamage`
  (params (Damage :type "Float (single-precision)") (DamageType :type "DamageType Object Reference") (InstigatedBy :type "Controller Object Reference") (DamageCauser :type "Actor Object Reference"))
  (`self.SetActorScale3D` (* (`self.GetActorScale3D`) 0.9))
  (bind _output_get (set `self.HP` (- (`self.HP`) Damage)))
  (if (<= _output_get 0.1)
    (`self.K2_DestroyActor`)))

(fn `UserConstructionScript`)